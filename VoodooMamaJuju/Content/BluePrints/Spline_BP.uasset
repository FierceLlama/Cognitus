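; Spline-driven actor that lays a neuron path mesh along its spline.
; The construction script divides the spline length by Spacing and adds one material-assigned spline mesh component per step.
; Each segment takes world-space positions and directions at its two distances, with tangents scaled by TangentSpacing, using manual attachment for the components.
; The event graph has no runtime logic.
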(event `self.ReceiveBeginPlay`)

(event `self.ReceiveActorBeginOverlap`
  (params (OtherActor :type "Actor Object Reference")))

(event `self.ReceiveTick`
  (params (DeltaSeconds :type "Float (single-precision)")))

(fn `UserConstructionScript`
  (bind _tangentspacing (`self.tangentSpacing`))
  (bind _splinecomponent (`self.SplineComponent`))
  (bind _spacing (`self.spacing`))
  (for _index (range (+ (`.ReturnValue` (`KismetMathLibrary.FMod` (`SplineComponent.GetSplineLength` _splinecomponent) _spacing)) 1))
    (bind _returnvalue (`AddComponent|Spline Mesh Component_8319` :`bManualAttachment` true))
    (`StaticMeshComponent.SetStaticMesh` _returnvalue "/Game/Assets/StaticMeshes/Neuron_Path.Neuron_Path")
    (`PrimitiveComponent.SetMaterial` _returnvalue 0 "/Game/Assets/StaticMeshes/lambert1.lambert1")
    (bind _returnvalue_2 (* _index _spacing))
    (bind _returnvalue_3 (+ _returnvalue_2 _spacing))
    (`SplineMeshComponent.SetStartAndEnd` _returnvalue (`SplineComponent.GetLocationAtDistanceAlongSpline` _splinecomponent _returnvalue_2 "World") (* (`SplineComponent.GetDirectionAtDistanceAlongSpline` _splinecomponent _returnvalue_2 "World") _tangentspacing) (`SplineComponent.GetLocationAtDistanceAlongSpline` _splinecomponent _returnvalue_3 "World") (* (`SplineComponent.GetDirectionAtDistanceAlongSpline` _splinecomponent _returnvalue_3 "World") _tangentspacing))))