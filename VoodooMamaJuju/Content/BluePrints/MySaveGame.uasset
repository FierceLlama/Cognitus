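; MySaveGame Blueprint that tracks the player's highest time through Save and Load functions.
; Save loads the slot named on SaveGameInstance, keeps the larger time or creates a new object if loading fails, but never writes to the slot.
; Load reads the same slot and returns PlayerTime.
; The EventGraph code that would initialize SaveGameInstance never runs, yet both functions read slot details from it first.
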(fn `Load`
  (returns (TopPlayerTime :type "Float (double-precision)"))
  (bind _savegameinstance (`self.SaveGameInstance`))
  (bind _returnvalue (`GameplayStatics.LoadGameFromSlot` (`/Game/BluePrints/MySaveGame.SaveSlotName` _savegameinstance) (`/Game/BluePrints/MySaveGame.UserIndex` _savegameinstance)))
  (bind _asmy_save_game (cast `/Game/BluePrints/MySaveGame` _returnvalue))
  (bind _output_get (set `self.SaveGameInstance` _asmy_save_game))
  (return (`/Game/BluePrints/MySaveGame.PlayerTime` _output_get)))

(fn `Save`
  (params (GameTime :type "Float (double-precision)"))
  (bind _savegameinstance (`self.SaveGameInstance`))
  (bind _returnvalue (`GameplayStatics.LoadGameFromSlot` (`/Game/BluePrints/MySaveGame.SaveSlotName` _savegameinstance) (`/Game/BluePrints/MySaveGame.UserIndex` _savegameinstance)))
  (bind _asmy_save_game (cast `/Game/BluePrints/MySaveGame` _returnvalue)
    (:`then`
      (bind _output_get (set `self.SaveGameInstance` _asmy_save_game))
      (if (> GameTime (`/Game/BluePrints/MySaveGame.PlayerTime` _output_get))
        (set `/Game/BluePrints/MySaveGame.PlayerTime` GameTime _output_get)))
    (:`CastFailed`
      (bind _returnvalue_2 (`GameplayStatics.CreateSaveGameObject` "MySaveGame_C"))
      (bind _asmy_save_game_2 (cast `/Game/BluePrints/MySaveGame` _returnvalue_2))
      (bind _output_get_2 (set `self.SaveGameInstance` _asmy_save_game_2))
      (set `/Game/BluePrints/MySaveGame.PlayerTime` GameTime _output_get_2))))