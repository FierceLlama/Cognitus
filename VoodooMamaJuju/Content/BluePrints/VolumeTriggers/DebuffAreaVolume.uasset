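; Trigger volume that debuffs the player while inside its area.
; On BeginPlay it caches actors of class NewPlayerControls_BPC and treats the first as the player, ignoring other overlapping actors.
; Entering runs the trigger overlap implementation, then calls Debuff on the player unless InDebuffZone is already set.
; Leaving calls SetLastingDebuff, leaving the effect logic to the player Blueprint.
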(event `self.ReceiveBeginPlay`
  (bind _outactors (`GameplayStatics.GetAllActorsOfClass` "/Game/Entities/Player/NewPlayerControls_BPC.NewPlayerControls_BPC_C"))
  (set `self.player` _outactors))

(event `self.OnBeginTriggerOverlap`
  (params (OtherActor :type "Actor Object Reference") (OtherComp :type "PrimitiveComponent Object Reference") (OtherBodyIndex :type Integer) (bFromSweep :type Boolean) (SweepResult :type "HitResult Structure (by ref)"))
  (bind _item (`KismetArrayLibrary.Array_Get` (`self.player`)))
  (if (== OtherActor _item)
    (`self.OnBeginTriggerOverlap_Implementation` null null 0 false SweepResult)
    (if (not (`/Game/Entities/Player/NewPlayerControls_BPC.inDebuffZone` _item))
      (`/Game/Entities/Player/NewPlayerControls_BPC.Debuff` _item))))

(event `self.OnEndTriggerOverlap`
  (params (OtherActor :type "Actor Object Reference") (OtherComp :type "PrimitiveComponent Object Reference") (OtherBodyIndex :type Integer))
  (bind _item (`KismetArrayLibrary.Array_Get` (`self.player`)))
  (if (== OtherActor _item)
    (`/Game/Entities/Player/NewPlayerControls_BPC.SetLastingDebuff` _item)))

(fn `UserConstructionScript`)