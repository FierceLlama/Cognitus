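; BP_HazardTriggerBlueprint is a trigger Blueprint for a slow-zone hazard that is currently inactive, as both overlap events are empty.
; Two disconnected chains find the first IncreasingSpeed_BPC actor and overwrite its DebuffThrust.
; The entry chain divides Thrust by DebuffThrust and the exit chain multiplies them, each printing a zone message.
; The construction script is empty.
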(event `self.OnBeginTriggerOverlap`
  (params (OtherActor :type "Actor Object Reference") (OtherComp :type "PrimitiveComponent Object Reference") (OtherBodyIndex :type Integer) (bFromSweep :type Boolean) (SweepResult :type "HitResult Structure (by ref)"))
  ;[1 1 1] Begin Overlap
)

(event `self.OnEndTriggerOverlap`
  (params (OtherActor :type "Actor Object Reference") (OtherComp :type "PrimitiveComponent Object Reference") (OtherBodyIndex :type Integer))
  ;[1 1 1] End Overlap
)

(fn `UserConstructionScript`)