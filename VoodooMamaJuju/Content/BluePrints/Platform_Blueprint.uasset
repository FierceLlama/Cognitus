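; Platform Blueprint actor that builds a platform shape along a spline.
; The construction script adds one spline mesh component per segment between adjacent spline points and attaches it to TopScene.
; Each segment takes its local start and end locations and tangents from the spline, with both tangents multiplied by TangentScale to adjust curvature.
; The event graph has no runtime logic, including an empty spline overlap event.
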(event `self.ReceiveBeginPlay`)

(event `self.ReceiveActorBeginOverlap`
  (params (OtherActor :type "Actor Object Reference")))

(event `self.ReceiveTick`
  (params (DeltaSeconds :type "Float (single-precision)")))

(event `self.Spline.OnComponentBeginOverlap`
  (params (OtherActor :type "Actor Object Reference") (OtherComp :type "PrimitiveComponent Object Reference") (OtherBodyIndex :type Integer) (bFromSweep :type Boolean) (SweepResult :type "HitResult Structure (by ref)")))

(fn `UserConstructionScript`
  (bind _tangentscale (`self.tangentScale`))
  (bind _spline (`self.Spline`))
  (for _index (range (+ (- (`SplineComponent.GetNumberOfSplinePoints` (`self.Spline`)) 2) 1))
    (bind _returnvalue (`AddComponent|Spline Mesh Component_0` :`bManualAttachment` true))
    (`SceneComponent.K2_AttachTo` _returnvalue (`self.Top_Scene`) "None" "KeepRelativeOffset" true)
    (bind (_location _tangent) (`SplineComponent.GetLocationAndTangentAtSplinePoint` _spline _index "Local"))
    (bind (_location_2 _tangent_2) (`SplineComponent.GetLocationAndTangentAtSplinePoint` _spline (+ _index 1) "Local"))
    (`SplineMeshComponent.SetStartAndEnd` _returnvalue _location (* _tangent _tangentscale) _location_2 (* _tangent_2 _tangentscale))))